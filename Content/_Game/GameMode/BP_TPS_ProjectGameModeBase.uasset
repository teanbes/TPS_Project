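; Game mode for a third-person project that tracks score and triggers the win screen when all enemies are accounted for.
; Shortly after BeginPlay it sets game-only input and counts the BP_Enemy actors in the level as the max score.
; Each AddScore call increments the score; on reaching the max it shows WBP_EndScreen, switches to UI input with the cursor visible and ignores player movement.
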(event Custom|AddScore
  (bind _returnvalue (Game|GetPlayerController 0))
  (Math|Integer|IncrementInt (Variables|Default|GetCurrentScore) ; Update Score
    (:%20%20
      (if (== (Variables|Default|GetCurrentScore) (Variables|Default|GetMaxScore)) ; Win Condition
        ;[1 1 1] Win Panel Widget
        (bind _returnvalue_2 (UserInterface|CreateWidget "/Game/_Game/HUD/WBP_EndScreen.WBP_EndScreen_C"))
        (UserInterface|Viewport|AddtoViewport _returnvalue_2 0)
        ;[1 1 1] Ignoring player movement and setting input mode to UI
        (Input|SetInputModeUIOnly _returnvalue _returnvalue_2 "DoNotLock" true)
        (Variables|/Script/Engine.PlayerController|SetbShowMouseCursor _returnvalue true)
        (Input|SetIgnoreMoveInput _returnvalue true)))))

(event EventBeginPlay
  (Utilities|FlowControl|Delay 0.5)
  (Input|SetInputModeGameOnly (Game|GetPlayerController 0) false)
  (bind _outactors (Actor|GetAllActorsOfClass "/Game/_Game/Enemies/BP_Enemy.BP_Enemy_C"))
  (Variables|Default|SetMaxScore (Utilities|Array|Length _outactors)))

(event EventTick
  (params (DeltaSeconds :type Float%20%28single-precision%29)))

(fn ConstructionScript)