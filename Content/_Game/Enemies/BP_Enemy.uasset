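; BP_Enemy is an enemy Blueprint with an overhead health bar widget that awards score on death.
; BeginPlay links the BP_EnemyHealthBar widget to the enemy and hides it.
; ShowHealthBar reveals the bar and then calls the parent implementation.
; HideHealthBar hides the bar and also calls AddScore on BP_TPS_ProjectGameModeBase, so kill scoring rides on that event.
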(event EventBeginPlay
  (bind _asbp_enemy_health_bar (Utilities|Casting|CastToBP_EnemyHealthBar (UserInterface|GetUserWidgetObject (Variables|Default|GetHealthBar))))
  (Variables|/Game/_Game/HUD/BP_EnemyHealthBar.BP_EnemyHealthBar_C|SetEnemy _asbp_enemy_health_bar self)
  (Widget|SetVisibility (UserInterface|GetUserWidgetObject (Variables|Default|GetHealthBar)) "Hidden"))

(event Collision|EventActorBeginOverlap
  (params (OtherActor :type Actor%20Object%20Reference)))

(event EventShowHealthBar
  ;[1 1 1] sets the timer for health bar visibility, triggers visibility
  (Widget|SetVisibility (UserInterface|GetUserWidgetObject (Variables|Default|GetHealthBar)) "Visible")
  (|CallParentFunction))

(event EventHideHealthBar
  ;[1 1 1] Resets timer,
  (Widget|SetVisibility (UserInterface|GetUserWidgetObject (Variables|Default|GetHealthBar)) "Hidden")
  ;[1 1 1] Add 1 to score after killing enemy
  (bind _asbp_tps_project_game_mode_base (Utilities|Casting|CastToBP_TPS_ProjectGameModeBase (Game|GetGameMode)))
  (Default|AddScore _asbp_tps_project_game_mode_base))

(fn ConstructionScript)