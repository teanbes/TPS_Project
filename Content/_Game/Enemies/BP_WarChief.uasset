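; BP_WarChief is an enemy Blueprint that manages the visibility of its floating health bar.
; On BeginPlay it runs the parent logic, links itself to the BP_EnemyHealthBar widget and hides it.
; ShowHealthBar reveals the widget before calling the parent event, while HideHealthBar hides it without a parent call.
; A disconnected node chain for adding score on a kill never runs.
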(event EventBeginPlay
  (|CallParentFunction)
  (bind _asbp_enemy_health_bar (Utilities|Casting|CastToBP_EnemyHealthBar (UserInterface|GetUserWidgetObject (Variables|Default|GetHealthBar))))
  (Variables|/Game/_Game/HUD/BP_EnemyHealthBar.BP_EnemyHealthBar_C|SetEnemy _asbp_enemy_health_bar self)
  (Widget|SetVisibility (UserInterface|GetUserWidgetObject (Variables|Default|GetHealthBar)) "Hidden"))

(event Collision|EventActorBeginOverlap
  (params (OtherActor :type Actor%20Object%20Reference)))

(event EventShowHealthBar
  ;[1 1 1] sets the timer for health bar visibility, triggers visibility
  (Widget|SetVisibility (UserInterface|GetUserWidgetObject (Variables|Default|GetHealthBar)) "Visible")
  (|CallParentFunction))

(event EventHideHealthBar
  ;[1 1 1] Resets timer,
  (Widget|SetVisibility (UserInterface|GetUserWidgetObject (Variables|Default|GetHealthBar)) "Hidden"))

(fn ConstructionScript)