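; BP_Health is a health pickup that heals the player on touch.
; When its sphere overlaps a BP_PlayerCharacter, it adds HealingPower to the character's Health, clamped to MaxHealth.
; It then plays a pickup sound at its location and destroys itself, even if the player was already at full health.
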(event OnComponentBeginOverlap(Sphere)
  (params (OverlappedComponent :type Primitive%20Component%20Object%20Reference) (OtherActor :type Actor%20Object%20Reference) (OtherComp :type Primitive%20Component%20Object%20Reference) (OtherBodyIndex :type Integer) (bFromSweep :type Boolean) (SweepResult :type Hit%20Result%20Structure%20%28by%20ref%29))
  ;[1 1 1] Health PickUp
  (bind _asbp_player_character (Utilities|Casting|CastToBP_PlayerCharacter OtherActor))
  (if (> (+ (Variables|/Script/TPS_Project.PlayerCharacter|GetHealth _asbp_player_character) (Variables|Default|GetHealingPower)) (Variables|/Script/TPS_Project.PlayerCharacter|GetMaxHealth _asbp_player_character))
    (Variables|/Script/TPS_Project.PlayerCharacter|SetHealth _asbp_player_character (Variables|/Script/TPS_Project.PlayerCharacter|GetMaxHealth _asbp_player_character))
    (else
      (Variables|/Script/TPS_Project.PlayerCharacter|SetHealth _asbp_player_character (+ (Variables|/Script/TPS_Project.PlayerCharacter|GetHealth _asbp_player_character) (Variables|Default|GetHealingPower)))))
  (Audio|PlaySoundatLocation (Variables|Default|GetHealthPickUpSound) (Transformation|GetActorLocation) "0, 0, 0" 1.0 1.0 0.0 0 0 0 0)
  (Actor|DestroyActor))

(fn ConstructionScript)